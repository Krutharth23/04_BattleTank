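; Player-controllable tank pawn Blueprint that binds aiming, driving and firing input to its tank components.
; On BeginPlay it registers the barrel and turret and initialises TankMovement with both tracks.
; Aim axes rotate an azimuth gimbal and spring arm, separate from the turret and barrel.
; Driving works either through per-track throttles or forward and rotate intents sent to TankMovement, while the fire action calls Fire.
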(event EventBeginPlay
  (Class|Tank|SetBarrelReference (Variables|Default|GetTankBarrel))
  (Class|Tank|SetTurretReference (Variables|Default|GetTankTurret))
  (Class|TankMovementComponent|Initialise (Variables|Default|GetTankMovement) (Variables|Default|GetTankTrackLeft) (Variables|Default|GetTankTrackRight)))

(event Input|ActionEvents|InputActionfire
  (params (Key :type Key%20Structure))
  ;[1 1 1] aim setup
  (:Pressed
    (Class|Tank|Fire)))

(event Input|AxisEvents|InputAxisAimAzimuth
  (params (AxisValue :type Float%20%28single-precision%29))
  ;[1 1 1] aim setup
  (Transformation|AddLocalRotation (Variables|Default|GetAzimuthGimbal) (Math|Rotator|MakeRotator 0.0 0.0 AxisValue) false false))

(event Input|AxisEvents|InputAxisrotate
  (params (AxisValue :type Float%20%28single-precision%29))
  (Class|TankMovementComponent|IntendRotate (Variables|Default|GetTankMovement) AxisValue))

(event Input|AxisEvents|InputAxisAimElevation
  (params (AxisValue :type Float%20%28single-precision%29))
  ;[1 1 1] aim setup
  (Transformation|AddLocalRotation (Variables|Default|GetSpringArm) (Math|Rotator|MakeRotator 0.0 AxisValue 0.0) false false))

(event Input|AxisEvents|InputAxisleftTrackThrottle
  (params (AxisValue :type Float%20%28single-precision%29))
  (Class|TankTrack|SetThrottle (Variables|Default|GetTankTrackLeft) AxisValue))

(event Input|AxisEvents|InputAxisRightTrackThrottle
  (params (AxisValue :type Float%20%28single-precision%29))
  (Class|TankTrack|SetThrottle (Variables|Default|GetTankTrackRight) AxisValue))

(event Input|AxisEvents|InputAxisMoveForward
  (params (AxisValue :type Float%20%28single-precision%29))
  (Class|TankMovementComponent|IntendMoveForward (Variables|Default|GetTankMovement) AxisValue))

(fn ConstructionScript)